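; Desktop character pawn that animates a torso mesh to follow the head and toggles an exit menu.
; Each tick, the torso smoothly interpolates toward the head's yaw, with pitch and roll kept level.
; The T key flips a visibility flag in BP_GameInstance_Main, either spawning BP_FinishWidget at an anchor transform, upright with matching yaw, or destroying all instances of it.
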(event `self.ReceiveTick`
  (params (DeltaSeconds :type "Float (single-precision)"))
  (bind _smesh_framework_torso (`self.SMesh_Framework_Torso`))
  (bind (_returnvalue_roll _returnvalue_pitch _returnvalue_yaw) (`KismetMathLibrary.BreakRotator` (`SceneComponent.K2_GetComponentRotation` (`self.Head`))))
  (`parent.ReceiveTick` DeltaSeconds)
  (`SceneComponent.K2_SetWorldRotation` _smesh_framework_torso (`KismetMathLibrary.RInterpTo` (`SceneComponent.K2_GetComponentRotation` _smesh_framework_torso) (`KismetMathLibrary.MakeRotator` 0.0 0.0 _returnvalue_yaw) DeltaSeconds 2.0) false false))

(event `InputAction|Keyboard_T`
  (params (Key :type "Key Structure"))
  (bind _returnvalue (`SceneComponent.K2_GetComponentToWorld` (`self.FinishWidgetTransform`)))
  ;[1 1 1] ExitMenu toggle
  (:`Pressed`
    (bind _asbp_game_instance_main (cast `/Game/AFCore/Blueprints/Game/BP_GameInstance_Main` (`GameplayStatics.GetGameInstance`)))
    (if (`/Game/AFCore/Blueprints/Game/BP_GameInstance_Main.IsInstanceFinishVisible` _asbp_game_instance_main)
      (set `/Game/AFCore/Blueprints/Game/BP_GameInstance_Main.IsInstanceFinishVisible` false _asbp_game_instance_main)
      (bind _outactors (`GameplayStatics.GetAllActorsOfClass` "/Game/AFCore/Blueprints/UI/Utils/BP_FinishWidget.BP_FinishWidget_C"))
      (`self.K2_DestroyActor` _outactors)
      (else
        (set `/Game/AFCore/Blueprints/Game/BP_GameInstance_Main.IsInstanceFinishVisible` true _asbp_game_instance_main)
        (`|SpawnActorFromClass` "/Game/AFCore/Blueprints/UI/Utils/BP_FinishWidget.BP_FinishWidget_C" (`KismetMathLibrary.MakeTransform` (.location _returnvalue) (`KismetMathLibrary.MakeRotator` 0.0 0.0 (.yaw (.rotation _returnvalue))) (.scale _returnvalue)) "Undefined" "OverrideRootScale" null null)))))

(fn `UserConstructionScript`
  (`parent.UserConstructionScript`))