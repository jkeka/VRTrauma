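; BP_GameManager is a manager Blueprint meant to record play time in the game instance.
; On EndPlay it casts to BP_GameInstance_Main and copies TotalSeconds into PlayTime0, printing an error if the cast fails.
; The GameTime accumulation, its rounding into TotalSeconds and a RealtimeTimer update are disconnected, and Tick is empty, so nothing here advances the saved value.
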(event `self.ReceiveBeginPlay`)

(event `self.ReceiveTick`
  (params (DeltaSeconds :type "Float (single-precision)")))

(event `self.ReceiveEndPlay`
  (params (EndPlayReason :type "EEndPlayReason Enum" :default "Destroyed"))
  ;[1 1 1] Cast timer to GameInstance_BP
  (bind _asbp_game_instance_main (cast `/Game/AFCore/Blueprints/Game/BP_GameInstance_Main` (`GameplayStatics.GetGameInstance`))
    (:`then`
      (set `/Game/AFCore/Blueprints/Game/BP_GameInstance_Main.playTime_0` (`self.totalSeconds`) _asbp_game_instance_main))
    (:`CastFailed`
      (`KismetSystemLibrary.PrintString` "GameManager to GameInstance cast failed"))))

(fn `UserConstructionScript`)