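; BP_Patient is a patient actor that shows an info widget when selected and accumulates a per-patient timer on Tick.
; Selection reveals the widget and yaws it once toward the player pawn.
; An overlap component sets the player-close flag and enables input on begin, then hides the widget on end without disabling input.
; BeginPlay hides the widget, stores and prints the location, and zeroes the game instance's checked-patient count.
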(event `self.ReceiveTick`
  (params (DeltaSeconds :type "Float (single-precision)"))
  (`|ExecutionSequence`
    (:`then_0`
      (set `self.PatientTimer` (+ DeltaSeconds (`self.PatientTimer`))))))

(event `self.Comp_Select.PressedSelect`
  (params (Pawn :type "/Game/AFCore/Blueprints/Pawn/BP_Pawn_Base Object Reference") (SourceActor :type "Actor Object Reference") (ImpactLocation :type "Vector Structure") (ImpactComponent :type "ActorComponent Object Reference"))
  (bind (_returnvalue_roll _returnvalue_pitch _returnvalue_yaw) (`KismetMathLibrary.BreakRotator` (`KismetMathLibrary.FindLookAtRotation` (`self.K2_GetActorLocation`) (`self.K2_GetActorLocation` (`GameplayStatics.GetPlayerPawn` 0)))))
  (set `self.isPatientWidgetVisible` true)
  (`SceneComponent.SetVisibility` (`self.Comp_Widget`) true false)
  ;[1 1 1] Make widget face player when coming visible
  (`SceneComponent.K2_SetWorldRotation` (`self.Comp_Widget`) (`KismetMathLibrary.MakeRotator` 0.0 0.0 _returnvalue_yaw) false false))

(event `self.Comp_Overlap_Comp.ActorBeginOverlap`
  (params (OtherActor :type "Actor Object Reference") (OtherComp :type "PrimitiveComponent Object Reference"))
  (set `self.isPlayerClose` true)
  (`self.EnableInput` (`GameplayStatics.GetPlayerController` 0)))

(event `self.ReceiveBeginPlay`
  (`|ExecutionSequence`
    (:`then_0`
      (`SceneComponent.SetVisibility` (`self.Comp_Widget`) false false))
    (:`then_1`
      (bind _output_get (set `self.PatientTransform` (`self.K2_GetActorLocation`)))
      (`KismetSystemLibrary.PrintString` (`KismetStringLibrary.Conv_VectorToString` _output_get) true true (struct :`R` 1.0 :`B` 0.091539 :`A` 1.0)))
    (:`then_2`
      (bind _asbp_game_instance_main (cast `/Game/AFCore/Blueprints/Game/BP_GameInstance_Main` (`GameplayStatics.GetGameInstance`))
        (:`then`
          (set `/Game/AFCore/Blueprints/Game/BP_GameInstance_Main.checkedPatientsCount` 0 _asbp_game_instance_main))
        (:`CastFailed`
          (`KismetSystemLibrary.PrintString` "GameManager to GameInstance cast failed"))))))

(event `self.Comp_Overlap_Comp.ActorEndOverlap`
  ;[1 1 1] Hide widget when not near
  (set `self.isPlayerClose` false)
  (`SceneComponent.SetVisibility` (`self.Comp_Widget`) false false)
  (set `self.isPatientWidgetVisible` false))

(fn `UserConstructionScript`)